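; Dash gameplay ability that launches the player character along the camera's forward vector while playing a dash montage.
; During the dash it zeroes ground friction and lets the capsule overlap pawns, restoring both and ending when the montage finishes or is interrupted.
; A dealDamage gameplay event applies a damage effect to the target, then pushes enemies away from the player, stuns them and draws a debug arrow.
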(event `self.K2_ActivateAbility`
  (bind _returnvalue (`Actor.K2_GetActorLocation` (`self.GetCharacterBaseAndPlayerController`)))
  (`self.K2_CommitAbility`)
  (bind _asbp_base_character (cast `/Game/Blueprints/Characters/BP_BaseCharacter` (`self.GetOwningActorFromActorInfo`))
    (:`then`
      (bind _charactermovement (`Character.CharacterMovement` _asbp_base_character))
      (set `self.OriginalGroundFriction` (`CharacterMovementComponent.GroundFriction` _charactermovement))
      (set `CharacterMovementComponent.GroundFriction` 0.0 _charactermovement)
      (`/Game/Blueprints/Characters/BP_BaseCharacter.SetCollisionToPawn` (`self.GetCharacterBaseAndPlayerController`) "ECR_Overlap")
      (`Character.LaunchCharacter` _asbp_base_character (* (`SceneComponent.GetForwardVector` (`/Game/Blueprints/Characters/BP_BaseCharacter.PlayerCamera` _asbp_base_character)) (`self.LaunchSpeed`)) false false)
      (`AbilityTask_PlayMontageAndWait.CreatePlayMontageAndWaitProxy` "None" "/Game/Blueprints/Characters/Animations/AM_DashAbility_Shinbi.AM_DashAbility_Shinbi"
        (:`then`
          (bind (_asynctaskproxy _payload) (`AbilityTask_WaitGameplayEvent.WaitGameplayEvent` (struct :`TagName` "ability.dash.dealDamage") null)
            (:`EventReceived`
              (bind (_eventtag _instigator _target) (break `GameplayEventData` _payload))
              (`self.BP_ApplyGameplayEffectToTarget` (`AbilitySystemBlueprintLibrary.AbilityTargetDataFromActor` _target) "/Game/Blueprints/Characters/Abilities/Dash/GE_Dash_DealDamage.GE_Dash_DealDamage_C")
              (bind _asbp_enemy (cast `/Game/Blueprints/Characters/BP_Enemy` _target))
              (bind _returnvalue_2 (`KismetMathLibrary.Normal` (- (`Actor.K2_GetActorLocation` _asbp_enemy) _returnvalue)))
              (`ASCharacterBase.PushCharacter` _asbp_enemy _returnvalue_2 10000.0)
              (`KismetSystemLibrary.DrawDebugArrow` _returnvalue (+ (* _returnvalue_2 400.0) _returnvalue) 8.0 (struct :`R` 200.0 :`B` 20.567226 :`A` 1.0) 4.0 6.0)
              (`ASCharacterBase.Stun` _asbp_enemy 5.0))))
        (:`OnCompleted`
          (set `CharacterMovementComponent.GroundFriction` (`self.OriginalGroundFriction`) _charactermovement :!label _label)
          (`/Game/Blueprints/Characters/BP_BaseCharacter.SetCollisionToPawn` (`self.GetCharacterBaseAndPlayerController`) "ECR_Block")
          (`self.K2_EndAbility`))
        (:`OnBlendOut`
          (goto _label))
        (:`OnInterrupted`
          (goto _label))
        (:`OnCancelled`
          (goto _label))))
    (:`CastFailed`
      (`self.K2_EndAbility`))))