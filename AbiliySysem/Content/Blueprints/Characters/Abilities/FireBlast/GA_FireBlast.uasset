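; GA_FireBlast is a gameplay ability that pulls surrounding characters toward the caster, then blasts them away with damage.
; A cast montage drives it through gameplay events, and the ability ends when the montage finishes or breaks off.
; The pull event gathers targets instantly in a radius via GATargetActorGetAround, caches them and applies an inward push-and-stun.
; The push event reuses those targets for the damage effect and an outward push-and-stun.
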(event `self.K2_ActivateAbility`
  (bind _targetdatahandle (`self.TargetDataHandle`))
  (`AbilityTask_PlayMontageAndWait.CreatePlayMontageAndWaitProxy` "None" "/Game/Blueprints/Characters/Animations/AM_FireBlast_Cast.AM_FireBlast_Cast"
    (:`then`
      (`AbilityTask_WaitGameplayEvent.WaitGameplayEvent` (struct :`TagName` "ability.fireBlast.pull") null
        (:`EventReceived`
          (bind (_asynctaskproxy _data) (`AbilityTask_WaitTargetData.WaitTargetData` "None" "Instant" "/Script/AbiliySysem.GATargetActorGetAround" 800.0 (struct) (struct) null)
            (:`then`
              (`AbilityTask_WaitGameplayEvent.WaitGameplayEvent` (struct :`TagName` "ability.fireBlast.push") null
                (:`EventReceived`
                  (`self.BP_ApplyGameplayEffectToTarget` _targetdatahandle "/Game/Blueprints/Characters/Abilities/FireBlast/GE_FireBlast_Damage.GE_FireBlast_Damage_C")
                  (for _array_element (`AbilitySystemBlueprintLibrary.GetActorsFromTargetData` _targetdatahandle)
                    (bind _asbp_base_character (cast `/Game/Blueprints/Characters/BP_BaseCharacter` _array_element))
                    (bind _returnvalue (`KismetMathLibrary.Normal` (- (`Actor.K2_GetActorLocation` (`self.GetOwningActorFromActorInfo`)) (`Actor.K2_GetActorLocation` (stale _array_element_2)))))
                    (`/Game/Blueprints/Characters/BP_BaseCharacter.PushAndStun` _asbp_base_character (* _returnvalue -1.0) 2500.0 2.0 null)))))
            (:`ValidData`
              (set `self.TargetDataHandle` _data)
              (for _array_element_2 (`AbilitySystemBlueprintLibrary.GetActorsFromTargetData` _data)
                (bind _asbp_base_character_2 (cast `/Game/Blueprints/Characters/BP_BaseCharacter` _array_element_2))
                (`/Game/Blueprints/Characters/BP_BaseCharacter.PushAndStun` _asbp_base_character_2 _returnvalue 2000.0 3.0 null)))
            (:`Cancelled`
              (`self.K2_EndAbility`))))))
    (:`OnCompleted`
      (`self.K2_EndAbility` :!label _label))
    (:`OnBlendOut`
      (goto _label))
    (:`OnInterrupted`
      (goto _label))
    (:`OnCancelled`
      (goto _label))))