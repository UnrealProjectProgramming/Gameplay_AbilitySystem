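; Fireball ability projectile that applies a gameplay effect to hostile characters it hits.
; On sphere overlap, it casts the target and its instigator to BP_BaseCharacter and checks hostility between them.
; For hostile targets, the instigator applies the ability-supplied effect spec through actor target data, then the projectile destroys itself.
; BeginPlay also binds self-destruction to a non-looping timer, but its time is zero.
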(event `self.ReceiveBeginPlay`
  (`KismetSystemLibrary.K2_SetTimerDelegate` (delegate `Destroy`)))

(event `Destroy`
  (`self.K2_DestroyActor`))

(event `self.Sphere.OnComponentBeginOverlap`
  (params (OverlappedComponent :type "PrimitiveComponent Object Reference") (OtherActor :type "Actor Object Reference") (OtherComp :type "PrimitiveComponent Object Reference") (OtherBodyIndex :type Integer) (bFromSweep :type Boolean) (SweepResult :type "HitResult Structure (by ref)"))
  (bind _asbp_base_character (cast `/Game/Blueprints/Characters/BP_BaseCharacter` OtherActor))
  (bind _asbp_base_character_2 (cast `/Game/Blueprints/Characters/BP_BaseCharacter` (`self.GetInstigator`)))
  (if (`ASCharacterBase.IsOtherHostile` _asbp_base_character _asbp_base_character_2)
    (`ASCharacterBase.ApplyGESpecHandleToTargetDataSpecHandle` _asbp_base_character_2 (`self.EffectSpecHandleFromAbility`) (`AbilitySystemBlueprintLibrary.AbilityTargetDataFromActor` OtherActor))
    (`self.K2_DestroyActor`)))

(fn `UserConstructionScript`)