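; Laser beam actor for an ability that repeatedly reports hostile characters touching the beam's end so they can be damaged.
; Each tick it drives an end-bone offset in the skeletal mesh's AnimBP, stretching the beam to match the distance to LazerEndDetector.
; Detector overlaps maintain a list of characters hostile to the instigator.
; A looping timer sends that list to the instigator as target data in an Ability.lazer.dealDamage gameplay event.
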(event `self.ReceiveBeginPlay`
  (set `self.BeamOriginalLength` (`KismetMathLibrary.VSize` (- (`SceneComponent.GetSocketLocation` (`self.LazerSkeletalMesh`) "end") (`self.K2_GetActorLocation`))))
  ;[1 1 1] Send Damage Event Every 0.3 Second
  (`KismetSystemLibrary.K2_SetTimerDelegate` (delegate `SendDealDamageEvent`) 0.2 true))

(event `SendDealDamageEvent`
  ;[1 1 1] Send Damage Event Every 0.3 Second
  (if (`KismetMathLibrary.Conv_IntToBool` (`KismetArrayLibrary.Array_Length` (`self.OverlappingActors`)))
    (`AbilitySystemBlueprintLibrary.SendGameplayEventToActor` (`self.GetInstigator`) (struct :`TagName` "ability.lazer.dealDamage") (make `GameplayEventData` (struct) null null null null (struct) (struct) (struct) 0.0 (`AbilitySystemBlueprintLibrary.AbilityTargetDataFromActorArray` (`self.OverlappingActors`))))))

(event `self.ReceiveTick`
  (params (DeltaSeconds :type "Float (single-precision)"))
  (bind _asanim_bp_lazer_skeletal_mesh_skeleton (cast `/Game/Blueprints/Characters/Abilities/Lazer/Assets/AnimBP_lazer_skeletal_mesh_Skeleton` (`SkeletalMeshComponent.GetAnimInstance` (`self.LazerSkeletalMesh`))))
  (set `/Game/Blueprints/Characters/Abilities/Lazer/Assets/AnimBP_lazer_skeletal_mesh_Skeleton.EndBoneOffset` (`KismetMathLibrary.MakeVector` (- (`KismetMathLibrary.VSize` (- (`SceneComponent.K2_GetComponentLocation` (`self.LazerEndDetector`)) (`self.K2_GetActorLocation`))) (`self.BeamOriginalLength`))) _asanim_bp_lazer_skeletal_mesh_skeleton))

(event `self.LazerEndDetector.OnComponentBeginOverlap`
  (params (OverlappedComponent :type "PrimitiveComponent Object Reference") (OtherActor :type "Actor Object Reference") (OtherComp :type "PrimitiveComponent Object Reference") (OtherBodyIndex :type Integer) (bFromSweep :type Boolean) (SweepResult :type "HitResult Structure (by ref)"))
  (bind _asbp_base_character (cast `/Game/Blueprints/Characters/BP_BaseCharacter` OtherActor))
  (bind _asbp_base_character_2 (cast `/Game/Blueprints/Characters/BP_BaseCharacter` (`self.GetInstigator`)))
  (if (`ASCharacterBase.IsOtherHostile` _asbp_base_character_2 _asbp_base_character)
    (`KismetArrayLibrary.Array_AddUnique` (`self.OverlappingActors`) _asbp_base_character)))

(event `self.LazerEndDetector.OnComponentEndOverlap`
  (params (OverlappedComponent :type "PrimitiveComponent Object Reference") (OtherActor :type "Actor Object Reference") (OtherComp :type "PrimitiveComponent Object Reference") (OtherBodyIndex :type Integer))
  (bind _asbp_base_character (cast `/Game/Blueprints/Characters/BP_BaseCharacter` OtherActor))
  (`KismetArrayLibrary.Array_RemoveItem` (`self.OverlappingActors`) _asbp_base_character))

(fn `UserConstructionScript`)