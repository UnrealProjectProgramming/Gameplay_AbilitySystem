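; GA_Lazer is a Gameplay Ability that fires a lazer attack from the character.
; On activation it commits, starts the UI cooldown and plays the Shinbi lazer montage, then after a short delay enables camera control on the character.
; It spawns BP_Lazer attached to the mesh's Lazer socket, then waits for dealDamage gameplay events to apply GE_Lazer_DealDamage to their target data.
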(event `self.K2_ActivateAbility`
  (bind _characterbase (`self.GetCharacterBaseAndPlayerController`))
  (`self.K2_CommitAbility`)
  (`self.StartUICooldown`)
  (`AbilityTask_PlayMontageAndWait.CreatePlayMontageAndWaitProxy` "None" "/Game/Blueprints/Characters/Animations/AM_LazerAbility_Shinbi.AM_LazerAbility_Shinbi"
    (:`then`
      (`KismetSystemLibrary.Delay` 0.3)
      (`/Game/Blueprints/Characters/BP_BaseCharacter.ShouldCameraControl` _characterbase true)
      (bind (_asynctaskproxy _spawnedactor) (`AbilityTask_SpawnActor.SpawnActor` (struct) "/Game/Blueprints/Characters/Abilities/Lazer/BP_Lazer.BP_Lazer_C" _characterbase)
        (:`then`
          (`Actor.K2_AttachToComponent` _spawnedactor (`Character.Mesh` _characterbase) "Lazer" "SnapToTarget" "SnapToTarget" "KeepRelative" true)
          (bind (_asynctaskproxy_2 _payload) (`AbilityTask_WaitGameplayEvent.WaitGameplayEvent` (struct :`TagName` "ability.lazer.dealDamage") null)
            (:`EventReceived`
              (`self.BP_ApplyGameplayEffectToTarget` (`.TargetData` (break `GameplayEventData` _payload)) "/Game/Blueprints/Characters/Abilities/Lazer/GE_Lazer_DealDamage.GE_Lazer_DealDamage_C"))))))))