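; Player character Blueprint that ties Gameplay Ability System attributes to the player's HUD.
; On BeginPlay it applies the GE_Regen gameplay effect to itself through its ability system component.
; Health, mana and strength change events each cast the controller to BP_PlayerControllerBase and set the matching glass orb in the primary UI widget to the current-to-max ratio.
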(event `self.ReceiveBeginPlay`
  (`parent.ReceiveBeginPlay`)
  (`AbilitySystemComponent.BP_ApplyGameplayEffectToSelf` :`self` (`self.AbilitySystemComp`) :`GameplayEffectClass` "/Game/Blueprints/Characters/Abilities/BasicGameplayAbilities/GE_Regen.GE_Regen_C"))

(event `self.BP_OnHealthChanged`
  (params (Health :type "Float (single-precision)") (MaxHealth :type "Float (single-precision)"))
  ;[1 1 1] Updating UI for health, mana and strength
  (bind _asbp_player_controller_base (cast `/Game/Blueprints/BP_PlayerControllerBase` (`self.GetController`)))
  (`/Game/UI/WBP_GlassOrb.SetPercentage` (`/Game/UI/WBP_PrimaryUI.Health_GlassOrb` (`/Game/Blueprints/BP_PlayerControllerBase.PrimaryUIWidget` _asbp_player_controller_base)) (/ Health MaxHealth)))

(event `self.BP_OnManaChanged`
  (params (Mana :type "Float (single-precision)") (MaxMana :type "Float (single-precision)"))
  ;[1 1 1] Updating UI for health, mana and strength
  (bind _asbp_player_controller_base (cast `/Game/Blueprints/BP_PlayerControllerBase` (`self.GetController`)))
  (`/Game/UI/WBP_GlassOrb.SetPercentage` (`/Game/UI/WBP_PrimaryUI.Mana_GlassOrb` (`/Game/Blueprints/BP_PlayerControllerBase.PrimaryUIWidget` _asbp_player_controller_base)) (/ Mana MaxMana)))

(event `self.BP_OnStrengthChanged`
  (params (Strength :type "Float (single-precision)") (MaxStrength :type "Float (single-precision)"))
  ;[1 1 1] Updating UI for health, mana and strength
  (bind _asbp_player_controller_base (cast `/Game/Blueprints/BP_PlayerControllerBase` (`self.GetController`)))
  (`/Game/UI/WBP_GlassOrb.SetPercentage` (`/Game/UI/WBP_PrimaryUI.Strength_GlassOrb` (`/Game/Blueprints/BP_PlayerControllerBase.PrimaryUIWidget` _asbp_player_controller_base)) (/ Strength MaxStrength)))

(fn `UserConstructionScript`
  (`parent.UserConstructionScript`))