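; Base player controller Blueprint that turns player input into movement, camera, jump and attack actions on the possessed pawn.
; Move axes add movement input along the camera's forward and right vectors, while look axes feed controller pitch and yaw.
; Jump casts the pawn to Character, and the primary action casts it to BP_BaseCharacter to trigger a melee attack.
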(event `InputAxis|MoveForward`
  (params (AxisValue :type "Float (single-precision)"))
  ;[1 1 1] Basic Controll Setup
  (`Pawn.AddMovementInput` (`self.K2_GetPawn`) (`KismetMathLibrary.GetForwardVector` (`PlayerCameraManager.GetCameraRotation` (`self.PlayerCameraManager`))) AxisValue false))

(event `InputAxis|MoveRight`
  (params (AxisValue :type "Float (single-precision)"))
  ;[1 1 1] Basic Controll Setup
  (`Pawn.AddMovementInput` (`self.K2_GetPawn`) (`KismetMathLibrary.GetRightVector` (`PlayerCameraManager.GetCameraRotation` (`self.PlayerCameraManager`))) AxisValue false))

(event `InputAction|Jump`
  (params (Key :type "Key Structure"))
  ;[1 1 1] Basic Controll Setup
  (:`Pressed`
    (bind _ascharacter (cast `Character` (`self.K2_GetPawn`)))
    (`Character.Jump` _ascharacter)))

(event `InputAxis|LookUp`
  (params (AxisValue :type "Float (single-precision)"))
  ;[1 1 1] Basic Controll Setup
  (`self.AddPitchInput` AxisValue))

(event `InputAxis|LookRight`
  (params (AxisValue :type "Float (single-precision)"))
  ;[1 1 1] Basic Controll Setup
  (`self.AddYawInput` AxisValue))

(event `InputAction|PrimaryAction`
  (params (Key :type "Key Structure"))
  (:`Pressed`
    (bind _asbp_base_character (cast `/Game/Blueprints/Characters/BP_BaseCharacter` (`self.K2_GetPawn`)))
    (`/Game/Blueprints/Characters/BP_BaseCharacter.MeleeAttack` _asbp_base_character)))

(fn `UserConstructionScript`)